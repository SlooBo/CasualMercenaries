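; Player character Blueprint that connects keyboard input to the HUD's chat and shop and relays chat messages.
; After a short delay on BeginPlay, it caches the chat widget from BP_PlayerHud and hides its message element.
; UpdateChat passes messages through a server event, then a client event, into the chat widget.
; Enter toggles the chat textbox, B switches the HUD's shop element, and F1 flip-flops the mouse cursor.
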(event `self.ReceiveBeginPlay`
  (`KismetSystemLibrary.Delay` null 0.5)
  (bind _asbp_player_hud (cast `/Game/Game/Blueprints/BP_PlayerHud` (`PlayerController.GetHUD` (`GameplayStatics.GetPlayerController` null))))
  (bind _output_get (set `self.Chat` (`/Game/Game/Blueprints/BP_PlayerHud.Chat` _asbp_player_hud)))
  (`Widget.SetVisibility` (`/Game/ChatSystem/ChatWindow.Message` _output_get) "Hidden"))

(event `self.ReceiveActorBeginOverlap`
  (params (OtherActor :type "Actor Object Reference")))

(event `self.ReceiveTick`
  (params (DeltaSeconds :type "Float (single-precision)")))

(event `Update(client)`
  (params (message :type "/Game/ChatSystem/ChatMessageStruct Structure"))
  (`/Game/ChatSystem/ChatWindow.UpdateChat` (`self.Chat`) message))

(event `Update(server)`
  (params (message :type "/Game/ChatSystem/ChatMessageStruct Structure"))
  (`self.Update(client)` message))

(event `Key|Enter`
  (:`Pressed`
    (`/Game/ChatSystem/ChatWindow.Change Textbox Visibility` (`self.Chat`))))

(event `/Game/ChatSystem/Chat.Update Chat`
  (params (Message :type "/Game/ChatSystem/ChatMessageStruct Structure"))
  (`self.Update(server)` Message))

(event `Key|B`
  (:`Pressed`
    (bind _asbp_player_hud (cast `/Game/Game/Blueprints/BP_PlayerHud` (`PlayerController.GetHUD` (`GameplayStatics.GetPlayerController` null))))
    (`PlayerHud.changeUIElement` _asbp_player_hud "SHOP")))

(event `Key|F1`
  (bind _returnvalue (`GameplayStatics.GetPlayerController` null))
  (:`Pressed`
    (`/Engine/EditorBlueprintResources/StandardMacros.FlipFlop`
      (:`A`
        (set `PlayerController.bShowMouseCursor` true _returnvalue))
      (:`B`
        (set `PlayerController.bShowMouseCursor` false _returnvalue)))))

(fn `Get Player Name`
  (returns (Name :type String))
  (return (`PlayerState.PlayerName` (`self.PlayerState`))))

(fn `UserConstructionScript`)